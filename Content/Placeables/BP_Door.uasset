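; BP_Door is a placeable sliding double door that opens once when interacted with while unlocked.
; Interact checks IsLocked, then routes through DoOnce and OpeningDoor into ReplicateOpeningDoor, whose Opening timeline slides the two leaves apart along X.
; A separate event prints a debug string and calls ChangeMat, which turns a left-leaf material to green light and clears the lock.
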(event Custom|ChanginMaterials?
  (Development|PrintString "Hello")
  (CallFunction|ChangeMat))

(event Custom|ChangeMat
  (Rendering|Material|SetMaterial (Variables|Default|GetDoorLeft) 2 "/Game/SciFi_BioLaboratory/Materials/Objects/MI_Light_Green.MI_Light_Green")
  (Variables|Default|SetbIsLocked? false))

(event Custom|OpeningDoor
  (CallFunction|ReplicateOpeningDoor))

(event Custom|ReplicateOpeningDoor
  (bind _alpha (Timeline|Opening PlayFromStart)
    (:Update
      (Transformation|SetRelativeLocation (Variables|Default|GetDoorLeft) (Math|Vector|Lerp(Vector) "0, 0, 0" "-100.000000,0.000000,0.000000" _alpha) false false)
      (Transformation|SetRelativeLocation (Variables|Default|GetDoorRight) (Math|Vector|Lerp(Vector) "0, 0, 0" "100.000000,0.000000,0.000000" _alpha) false false))))

(event EventInteract
  (params (PlayerREF :type BP%20First%20Person%20Character%20Object%20Reference))
  (if (not (Variables|Default|GetbIsLocked?))
    (Utilities|FlowControl|DoOnce false
      (:Completed
        (CallFunction|OpeningDoor)))))

(fn ConstructionScript)