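; Interactable box that the player can grab and push or pull along its forward or right axis.
; Interact toggles the grab: it snaps the player beside the box, slows walking, switches move mode, locks look and toggles cube physics.
; While grabbed, a looping timer calls PushCabinet whenever the player moves.
; PushCabinet picks the axis best matching player velocity and sweeps the box toward the player's PushPullLoc on that axis, keeping height.
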(event Custom|StartMovingObject
  (Variables|Default|SetPlayerSKMesh (Variables|/Game/FirstPerson/Blueprints/BP_FirstPersonCharacter.BP_FirstPersonCharacter_C|GetFirstPersonMesh (.AsBP%20First%20Person%20Character (Utilities|Casting|CastToBP_FirstPersonCharacter (Game|Player|GetPlayerPawn 0)))))
  (bind _returnvalue (Utilities|Time|SetTimerbyEvent (delegate Custom|MoveObject) 0.01 true))
  (Variables|Default|SetMoveObjectHandle _returnvalue))

(event Custom|MoveObject
  (if (not (== (Math|Vector|VectorLength (Transformation|GetVelocity (Variables|Default|GetPlayerREF))) 0.0))
    (CallFunction|PushCabinet)))

(event Custom|StopMovingObject
  (bind _moveobjecthandle (Variables|Default|GetMoveObjectHandle))
  (if (Utilities|Time|IsValidTimerHandle _moveobjecthandle)
    (Utilities|Time|ClearandInvalidateTimerbyHandle _moveobjecthandle)))

(event EventInteract
  (params (PlayerREF :type BP%20First%20Person%20Character%20Object%20Reference))
  (|CallParentFunction PlayerREF)
  (if (Variables|Default|GetIsPlayerInteracting)
    (CallFunction|SetParameters false)
    (else
      (CallFunction|SetParameters true)
      (Transformation|SetActorLocation (Variables|Default|GetPlayerREF) (CallFunction|MakeLocation) false false)
      (Transformation|SetWorldRotation (Variables|/Script/Engine.Character|GetCapsuleComponent (Variables|Default|GetPlayerREF)) "0, 0, 0" false false))))

(fn ConstructionScript
  (|CallParentFunction))

(fn PushCabinet
  (bind _returnvalue (Transformation|GetActorForwardVector))
  (bind _returnvalue_2 (Transformation|GetActorRightVector))
  (bind _returnvalue_3 (Transformation|GetActorLocation))
  (bind _returnvalue_4 (Transformation|GetActorRightVector))
  (bind _returnvalue_5 (Transformation|GetActorForwardVector))
  (bind _playerref (Variables|Default|GetPlayerREF))
  (bind _playerref_2 (Variables|Default|GetPlayerREF))
  (bind _returnvalue_6 (Transformation|GetActorTransform _playerref_2))
  (bind _returnvalue_7 (Transformation|GetVelocity _playerref))
  (bind _pushpullloc (Variables|/Game/FirstPerson/Blueprints/BP_FirstPersonCharacter.BP_FirstPersonCharacter_C|GetPushPullLoc _playerref_2))
  (bind _returnvalue_8 (Math|Vector|Normalize _returnvalue_7))
  (bind _returnvalue_9 (Math|Transform|TransformLocation _returnvalue_6 _pushpullloc))
  (bind _returnvalue_10 (Math|Vector|DotProduct _returnvalue_4 _returnvalue_8))
  (bind _returnvalue_11 (Math|Vector|DotProduct _returnvalue_8 _returnvalue_5))
  (bind _returnvalue_12 (Math|Float|Absolute(Float) _returnvalue_11))
  (bind _returnvalue_13 (Math|Float|Absolute(Float) _returnvalue_10))
  (bind _returnvalue_14 (< _returnvalue_13 _returnvalue_12))
  (bind _returnvalue_15 (select _returnvalue_14 _returnvalue _returnvalue_2))
  (bind _returnvalue_16 (Math|Vector|VectorGetAbs _returnvalue_15))
  (bind (_x _y _z) (Math|Vector|BreakVector _returnvalue_15))
  (bind _returnvalue_17 (+ _returnvalue_16 -1.0))
  (bind _returnvalue_18 (* _returnvalue_9 _returnvalue_16))
  (bind _returnvalue_19 (+ _x _y _z))
  (bind _returnvalue_20 (Math|Vector|VectorGetAbs _returnvalue_17))
  (bind _returnvalue_21 (+ (.x _returnvalue_18) (.y _returnvalue_18) (.z _returnvalue_18)))
  (bind _returnvalue_22 (* 2e+01 _returnvalue_19))
  (bind _returnvalue_23 (* _returnvalue_20 _returnvalue_3))
  (bind _returnvalue_24 (+ _returnvalue_21 _returnvalue_22))
  (bind _returnvalue_25 (* _returnvalue_24 _returnvalue_16))
  (bind _returnvalue_26 (+ _returnvalue_25 _returnvalue_23))
  (Transformation|SetActorLocation (Math|Vector|MakeVector (.x _returnvalue_26) (.y _returnvalue_26) (.Z (Math|Vector|BreakVector _returnvalue_3))) true false))

(fn SetParameters
  (params (bIsFalse? :type Boolean))
  (bind _playerref (Variables|Default|GetPlayerREF))
  (Physics|SetSimulatePhysics (Variables|Default|GetCube) bIsFalse?)
  (Variables|Default|SetIsPlayerInteracting bIsFalse?)
  (Variables|/Script/Engine.CharacterMovementComponent|SetMaxWalkSpeed (Variables|/Script/Engine.Character|GetCharacterMovement (Variables|Default|GetPlayerREF)) (select bIsFalse? 2e+02 6e+02))
  (Variables|/Game/FirstPerson/Blueprints/BP_FirstPersonCharacter.BP_FirstPersonCharacter_C|SetMoveMode _playerref (select bIsFalse? 1 0))
  (Variables|/Game/FirstPerson/Blueprints/BP_FirstPersonCharacter.BP_FirstPersonCharacter_C|SetCanLook _playerref (not bIsFalse?))
  (if bIsFalse?
    (CallFunction|StartMovingObject)
    (else
      (CallFunction|StopMovingObject))))

(fn MakeLocation
  (bind _returnvalue (Transformation|GetActorRightVector))
  (bind _returnvalue_2 (Transformation|GetActorForwardVector))
  (bind _playerref (Variables|Default|GetPlayerREF))
  (bind _returnvalue_3 (Transformation|GetActorLocation _playerref))
  (bind _returnvalue_4 (Math|Vector|Normalize _returnvalue_3))
  (bind _returnvalue_5 (Math|Vector|DotProduct _returnvalue_4 _returnvalue))
  (bind _returnvalue_6 (Math|Vector|DotProduct _returnvalue_4 _returnvalue_2))
  (bind _returnvalue_7 (Math|Float|Absolute(Float) _returnvalue_6))
  (bind _returnvalue_8 (Math|Float|Absolute(Float) _returnvalue_5))
  (bind _returnvalue_9 (> _returnvalue_8 _returnvalue_7))
  (return (+ (* (* (select _returnvalue_9 _returnvalue _returnvalue_2) 1.5e+02) (select _returnvalue_9 (Math|Float|Ceil _returnvalue_5) (Math|Float|Ceil _returnvalue_6))) (Transformation|GetActorLocation))))