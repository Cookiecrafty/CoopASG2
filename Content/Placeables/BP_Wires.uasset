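; Interactable wire-cutting puzzle in which coloured wires are clicked to cut them.
; Interacting switches the view to this actor, enables mouse clicks and removes the player's HUD.
; Wire clicks call CutCable by colour name, which detaches the supplied cable's end and records the cut.
; Success is only a debug print, shown whenever every cut recorded so far matches the CablesToCut map.
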(event OnClicked(PurpleWire)
  (params (TouchedComponent :type Primitive%20Component%20Object%20Reference) (ButtonPressed :type Key%20Structure :default "None"))
  (CallFunction|CutCable (Utilities|Name|MakeLiteralName "Purple")))

(event OnClicked(GreenWire)
  (params (TouchedComponent :type Primitive%20Component%20Object%20Reference) (ButtonPressed :type Key%20Structure :default "None"))
  (CallFunction|CutCable (Utilities|Name|MakeLiteralName "Green")))

(event OnClicked(YellowWire)
  (params (TouchedComponent :type Primitive%20Component%20Object%20Reference) (ButtonPressed :type Key%20Structure :default "None"))
  (CallFunction|CutCable (Utilities|Name|MakeLiteralName "Yellow")))

(event OnClicked(BlueWire)
  (params (TouchedComponent :type Primitive%20Component%20Object%20Reference) (ButtonPressed :type Key%20Structure :default "None"))
  (CallFunction|CutCable (Utilities|Name|MakeLiteralName "Blue")))

(event OnClicked(RedWire)
  (params (TouchedComponent :type Primitive%20Component%20Object%20Reference) (ButtonPressed :type Key%20Structure :default "None"))
  (CallFunction|CutCable (Utilities|Name|MakeLiteralName "Red")))

(event OnClicked(Cube)
  (params (TouchedComponent :type Primitive%20Component%20Object%20Reference) (ButtonPressed :type Key%20Structure :default "None"))
  (Development|PrintString (Utilities|GetDisplayName TouchedComponent)))

(event EventInteract
  (params (PlayerREF :type BP%20First%20Person%20Character%20Object%20Reference))
  (bind _returnvalue (Game|GetPlayerController 0))
  (|CallParentFunction PlayerREF)
  (Variables|/Script/Engine.PlayerController|SetbEnableClickEvents _returnvalue true)
  (Game|Player|SetViewTargetwithBlend _returnvalue self 0.0 "VTBlend_Linear" 0.0 false)
  (Variables|/Script/Engine.PlayerController|SetbShowMouseCursor _returnvalue true)
  (Widget|RemovefromParent (Variables|/Game/FirstPerson/Blueprints/BP_FirstPersonCharacter.BP_FirstPersonCharacter_C|GetHUDRef (Variables|Default|GetPlayerREF))))

(fn ConstructionScript
  (|CallParentFunction))

(fn CutCable
  (params (WireName :type Name%20%28by%20ref%29) (WireToCut :type Cable%20Component%20Object%20Reference))
  (Variables|/Script/CableComponent.CableComponent|SetbAttachEnd WireToCut false)
  (Utilities|Map|Add (Variables|Default|GetCablesCut) WireName true)
  (bind (_keypin _valuepin) (Utilities|Map|ForEachLoop(Map) (Variables|Default|GetCablesCut) :!label _label)
    (:then
      (if (== (.Value (Utilities|Map|Find (Variables|Default|GetCablesToCut) _keypin)) _valuepin)
        (Variables|Default|SetSameWires true)
        (else
          (Variables|Default|SetSameWires false)
          (goto _label BreakPin))))
    (:CompletedPin
      (if (Variables|Default|GetSameWires)
        (Development|PrintString "yay !")))))