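; Interactable wire box puzzle where the player cuts wires to open linked doors.
; Interacting toggles a close-up view through the box, repositioning the player behind its camera and disabling movement.
; CutCable checks cuts against WiresToCut once two are made, calling OpeningDoors on the player if correct, otherwise disabling wire collision until a timed reset.
; The OpenDoors event changes materials on referenced doors and blocks further interaction.
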(event Custom|OpenDoors
  (for _array_element (Variables|Default|GetDoorRef)
    (Default|ChanginMaterials? _array_element)
    (Variables|Default|SetCanBeInteractedWith false)))

(event EventInteract
  (params (PlayerREF :type BP%20First%20Person%20Character%20Object%20Reference))
  (bind _returnvalue (Pawn|GetController PlayerREF))
  (bind _camera (Variables|Default|GetCamera))
  (bind _returnvalue_2 (Math|Vector|GetForwardVector _camera))
  (bind _returnvalue_3 (Transformation|GetWorldLocation _camera))
  (bind _asplayer_controller (Utilities|Casting|CastToPlayerController _returnvalue))
  (bind _charactermovement (Variables|/Script/Engine.Character|GetCharacterMovement (Variables|Default|GetPlayerREF)))
  (bind _returnvalue_4 (Math|Vector|MakeVector (.x _returnvalue_3) (.y _returnvalue_3) 0.0))
  (bind _returnvalue_5 (* _returnvalue_2 -5e+01))
  (bind _returnvalue_6 (+ _returnvalue_4 _returnvalue_5))
  (|CallParentFunction PlayerREF)
  (if (Variables|Default|GetCanBeInteractedWith)
    (if (Variables|Default|GetIsActive)
      (Variables|Default|SetIsActive false)
      (Game|Player|SetViewTargetwithBlend _asplayer_controller PlayerREF 0.0 "VTBlend_Linear" 0.0 false)
      (Default|LockRotation (Variables|Default|GetPlayerREF) true)
      (Pawn|Components|CharacterMovement|SetMovementMode _charactermovement "MOVE_Walking" 0)
      (else
        (Variables|Default|SetIsActive true)
        (Game|Player|SetViewTargetwithBlend _asplayer_controller self 0.0 "VTBlend_Linear" 0.0 false)
        (Transformation|SetActorLocation (Variables|Default|GetPlayerREF) (Math|Vector|MakeVector (.x _returnvalue_6) (.y _returnvalue_6) (.z (Transformation|GetActorLocation (Variables|Default|GetPlayerREF)))) false false)
        (Default|ControlRotationWires (Variables|Default|GetPlayerREF) (Transformation|GetWorldRotation (Variables|Default|GetCamera)))
        (Default|LockRotation (Variables|Default|GetPlayerREF) false)
        (Pawn|Components|CharacterMovement|DisableMovement _charactermovement)))))

(fn ConstructionScript
  (|CallParentFunction))

(fn CutCable
  (params (WireToCut :type BP%20Wire%20Object%20Reference))
  (bind _wirescut (Variables|Default|GetWiresCut))
  (Utilities|Array|Add _wirescut WireToCut)
  (if (>= (Utilities|Array|Length _wirescut) 2)
    (bind _array_element (Utilities|Array|ForEachLoopwithBreak (Variables|Default|GetWiresCut) :!label _label)
      (:LoopBody
        (if (!= (Utilities|Array|FindItem (Variables|Default|GetWiresToCut) _array_element) -1)
          (Variables|Default|SetisCorrect true)
          (else
            (Variables|Default|SetisCorrect false)
            (goto _label Break))))
      (:Completed
        (if (Variables|Default|GetisCorrect)
          (Default|OpeningDoors (Variables|Default|GetPlayerREF) self)
          (else
            (Utilities|FlowControl|Sequence
              (:then_0
                (for _array_element_2 (Variables|Default|GetWires)
                  (Utilities|IsValid _array_element_2
                    (:Is%20Valid
                      (Collision|SetActorEnableCollision _array_element_2 false)))))
              (:then_1
                (Utilities|Time|SetTimerbyFunctionName 0 "ResetWires" 1.0)))))))))

(fn ResetWires
  (bind _wirescut (Variables|Default|GetWiresCut))
  (for _array_element _wirescut
    (Default|Reset _array_element))
  (Utilities|Array|Clear _wirescut)
  (for _array_element_2 (Variables|Default|GetWires)
    (Utilities|IsValid _array_element_2
      (:Is%20Valid
        (Collision|SetActorEnableCollision _array_element_2 true)))))