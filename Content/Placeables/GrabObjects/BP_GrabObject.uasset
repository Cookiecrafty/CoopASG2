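; BP_GrabObject is a placeable physics object that the player can pick up by interacting with it.
; Interact releases anything the player already holds, enables physics on its Cube, then passes itself to the player's Grab function.
; While grabbed, the Cube ignores Pawn and Visibility collision channels, with a helper that can restore blocking.
; IsUsed destroys the actor.
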(event EventBeginPlay)

(event Collision|EventActorBeginOverlap
  (params (OtherActor :type Actor%20Object%20Reference)))

(event EventTick
  (params (DeltaSeconds :type Float%20%28single-precision%29)))

(event EventInteract
  (params (PlayerREF :type BP%20First%20Person%20Character%20Object%20Reference))
  (Variables|/Game/FirstPerson/Blueprints/BP_FirstPersonCharacter.BP_FirstPersonCharacter_C|GetGrabbedComponent PlayerREF
    (:then
      (Default|ReleaseGrabbedObject PlayerREF))
    (:else
      _))
  (Physics|SetSimulatePhysics (Variables|Default|GetCube) true)
  (CallFunction|SetCollisionResponsetoChannels true)
  (Default|Grab PlayerREF self))

(fn ConstructionScript)

(fn IsUsed
  (Actor|DestroyActor))

(fn SetCollisionResponsetoChannels
  (params (Grabbed? :type Boolean))
  (bind _returnvalue (select Grabbed? "ECR_Ignore" "ECR_Block"))
  (bind _cube (Variables|Default|GetCube))
  (Collision|SetCollisionResponsetoChannel _cube "ECC_Pawn" _returnvalue)
  (Collision|SetCollisionResponsetoChannel _cube "ECC_Visibility" _returnvalue))