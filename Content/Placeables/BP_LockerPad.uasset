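; BP_LockerPad is a placeable locker whose door swings open when OpenLocker is called.
; OpenLocker calls OpenMulti, which captures the door's rotation, sets the RepNotify Open flag, and plays a timeline that turns yaw up to 90 degrees.
; Interact is empty; the logic passing the pad and door code to the player's CodeLocker is disconnected, and OnRep_Open does nothing.
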(event Custom|Open%20Locker
  (CallFunction|OpenMulti))

(event Custom|Open%20Multi
  (Variables|Default|SetInitial%20rotation (Transformation|GetWorldRotation (Variables|Default|GetSM_Locker02Door01)))
  (Variables|Default|SetOpen? true)
  (bind _newtrack_0 (Timeline|Open PlayFromStart)
    (:Update
      (Transformation|SetWorldRotation (Variables|Default|GetSM_Locker02Door01) (Math|Rotator|MakeRotator (.roll (Variables|Default|GetInitial%20rotation)) (.pitch (Variables|Default|GetInitial%20rotation)) (+ (.yaw (Variables|Default|GetInitial%20rotation)) (* _newtrack_0 9e+01))) false false))))

(event EventInteract
  (params (PlayerREF :type BP%20First%20Person%20Character%20Object%20Reference)))

(fn ConstructionScript)

(fn OnRepOpen?)