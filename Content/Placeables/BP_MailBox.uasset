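; BP_MailBox is an interactable placeable mailbox that takes the player's held object and shuttles two mechanical doors.
; Interacting empty-handed toggles the doors, using a FlipFlop to play or reverse a timeline that slides them vertically in opposite directions.
; Interacting while holding something releases it, teleports it to the placement point and toggles the doors.
; That transfer disables interaction and blocks the box's Camera channel until the timeline finishes.
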(event Custom|MovingDoorsTimeline
  (Audio|PlaySoundatLocation "/Game/Sounds/SpaceShip/MechanicalDoor.MechanicalDoor" (Transformation|GetActorLocation) "0, 0, 0" 1.0 1.0 0.0 0 0 0 0)
  (Utilities|FlowControl|FlipFlop
    (:A
      (bind _alpha (Timeline|MovingDoors Play)
        (:Update
          (Transformation|SetRelativeLocation (Variables|Default|GetDoor1) (Math|Vector|Lerp(Vector) "-53.000000,45.000000,49.000000" "-53.000000,45.000000,180.000000" _alpha) false false)
          (Transformation|SetRelativeLocation (Variables|Default|GetDoor2) (Math|Vector|Lerp(Vector) "53.000000,-45.000000,180.000000" "53.000000,-45.000000,49.000000" _alpha) false false))
        (:Finished
          (Variables|Default|SetCanBeInteracted true)
          (Collision|SetCollisionResponsetoChannel (Variables|Default|GetBox) "ECC_Camera" "ECR_Ignore"))))
    (:B
      (Timeline|MovingDoors Reverse))))

(event Custom|SendObject
  (params (Target :type BP%20First%20Person%20Character%20Object%20Reference) (Target2 :type Actor%20Object%20Reference))
  (Variables|Default|SetCanBeInteracted false)
  (Variables|Default|SetbIsEmpty true)
  (Default|ReleaseObject Target)
  (Transformation|SetActorLocation Target2 (Transformation|GetWorldLocation (Variables|Default|GetWhereToPlaceObject)) false true)
  (CallFunction|MovingDoorsTimeline))

(event EventInteract
  (params (PlayerREF :type BP%20First%20Person%20Character%20Object%20Reference))
  (bind _grabbedcomponent (Variables|/Game/FirstPerson/Blueprints/BP_FirstPersonCharacter.BP_FirstPersonCharacter_C|GetGrabbedComponent PlayerREF))
  (|CallParentFunction PlayerREF)
  (if (Variables|Default|GetCanBeInteracted)
    (if (== _grabbedcomponent 0)
      (CallFunction|MovingDoorsTimeline)
      (else
        (Collision|SetCollisionResponsetoChannel (Variables|Default|GetBox) "ECC_Camera" "ECR_Block")
        (Variables|Default|SetObjectToExchange _grabbedcomponent)
        (CallFunction|SendObject PlayerREF (Variables|Default|GetObjectToExchange))))))

(fn ConstructionScript
  (|CallParentFunction))