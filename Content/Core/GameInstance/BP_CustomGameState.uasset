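; BP_CustomGameState is a game state that runs a bomb countdown and shows it on the player's HUD.
; On BeginPlay it casts the first controller's pawn to BP_FirstPersonCharacter, creates its HUD and starts a looping one-second timer.
; Each tick decrements TimerBomb only on the server, pushes it to that character, and stops the timer at zero.
; EndTimer, BombTimer and OnRep_TimerBomb are empty stubs.
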(event Custom|Start%20Bomb
  (bind _returnvalue (Utilities|Time|SetTimerbyEvent (delegate Custom|Bomb) 1.0 true))
  (Variables|Default|SetBombTimerFunction _returnvalue))

(event Custom|Bomb
  (if (Networking|IsServer)
    (bind _output_get (Variables|Default|SetTimerBomb (- (Variables|Default|GetTimerBomb) 1.0))))
  (Default|TimerUpdate (Variables|Default|GetPlayerRef) _output_get)
  (if (<= _output_get 0.0)
    (CallFunction|EndTimer)
    (Utilities|Time|ClearandInvalidateTimerbyHandle (Variables|Default|GetBombTimerFunction))))

(event EventBeginPlay
  (bind _asbp_first_person_character (Utilities|Casting|CastToBP_FirstPersonCharacter (Pawn|GetControlledPawn (Game|GetPlayerController 0))))
  (bind _output_get (Variables|Default|SetPlayerRef _asbp_first_person_character))
  (Default|CreateHUD _output_get)
  (CallFunction|StartBomb)
  (|CallParentFunction))

(fn ConstructionScript
  (|CallParentFunction))

(fn BombTimer)

(fn EndTimer)

(fn OnRepTimerBomb)